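; BP_TimeKeeper runs a hoverbike race: it creates the race HUD, counts down, then releases the player and AI racers.
; A looping timer drives the lap clock, and lap functions track previous and best times and format results.
; Half-second timers rank racers by spline distance plus lap count times track length, setting the player's position and, through a separate sort, every pawn's position.
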(event `self.ReceiveBeginPlay`
  (bind _outactors (`GameplayStatics.GetAllActorsOfClass` "/Game/Vehicles/Player/BP_BasePawn.BP_BasePawn_C"))
  (set `self.Racers` _outactors)
  (bind _asbp_hoverbike (cast `/Game/Vehicles/Player/BP_Hoverbike` (`GameplayStatics.GetPlayerPawn` 0)))
  (set `self.Player` _asbp_hoverbike)
  (bind _returnvalue (`|CreateWidget` "/Game/UI/WB_RaceHUD.WB_RaceHUD_C" (`GameplayStatics.GetPlayerController` 0)))
  (bind _output_get (set `self.RacingHUD` _returnvalue))
  (`UserWidget.AddToViewport` _output_get 0)
  (set `/Game/UI/WB_RaceHUD.Time Keeper` self _output_get)
  (bind _returnvalue_2 (`KismetSystemLibrary.K2_SetTimer` null "DecreaseCountdown" 1.0 true 1.0))
  (set `self.CountdownTimer` _returnvalue_2)
  (bind _returnvalue_3 (`KismetSystemLibrary.K2_SetTimer` null "GetPlayerPosition" 0.5 true))
  (set `self.PositionTimer` _returnvalue_3)
  (bind _returnvalue_4 (`KismetSystemLibrary.K2_SetTimer` null "GetRacerPositions" 0.5 true -0.5))
  (set `self.AIPositionTimer` _returnvalue_4)
  (bind _outactors_2 (`GameplayStatics.GetAllActorsOfClass` "/Game/Blueprints/BP_FinishMarker.BP_FinishMarker_C"))
  (bind _output_get_2 (set `self.FinishMarker` (`|GetArrayItem` _outactors_2)))
  (set `self.Lap to Finish` (`/Game/Blueprints/BP_FinishMarker.LapCountToFinish` _output_get_2)))

(event `StartRace`
  (bind _returnvalue (`KismetSystemLibrary.K2_SetTimer` null "StartTimer" 0.01 true))
  (set `self.LapTimer` _returnvalue)
  (bind _asbp_hoverbike (cast `/Game/Vehicles/Player/BP_Hoverbike` (`GameplayStatics.GetPlayerPawn` 0)))
  (set `/Game/Vehicles/Player/BP_Hoverbike.IsMovementEnabled?` true _asbp_hoverbike)
  (for _array_element (`self.AllRacers`)
    (set `/Game/Vehicles/AI/BP_AIRacer.HoldInPlace` false _array_element)))

(fn `Convert Time to Seconds`
  (returns (Seconds :type "Float (double-precision)"))
  (return (+ (/ (`KismetMathLibrary.Conv_IntToDouble` (`self.Miliseconds`)) 100.0) (`KismetMathLibrary.Conv_IntToDouble` (`self.Seconds`)) (* (`KismetMathLibrary.Conv_IntToDouble` (`self.Minutes`)) 60.0))))

(fn `ConvertLapResults`
  (params (LapResultMiliseconds :type Integer))
  (returns (ResultText :type String))
  (bind _returnvalue (`KismetMathLibrary.Conv_IntToDouble` (* LapResultMiliseconds 10)))
  (bind _returnvalue_2 (`KismetStringLibrary.Conv_IntToString` (`KismetMathLibrary.FFloor` (/ _returnvalue 60000.0))))
  (bind (_lefts _rights) (`KismetStringLibrary.Split` (`KismetStringLibrary.Conv_DoubleToString` (/ (mod _returnvalue 60000.0) 1000.0)) "."))
  (`|ExecutionSequence`
    (:`then_0`
      (if (< (`KismetStringLibrary.Conv_StringToInt` _returnvalue_2) 10)
        (set `self.MinutesResult` (`self.PadSingleDigit` _returnvalue_2))
        (else
          (set `self.MinutesResult` _returnvalue_2))))
    (:`then_1`
      (if (< (`KismetStringLibrary.Conv_StringToInt` _lefts) 10)
        (set `self.SecondsResults` (`self.PadSingleDigit` _lefts))
        (else
          (set `self.SecondsResults` _lefts))))
    (:`then_2`
      (if (< (`KismetStringLibrary.Conv_StringToInt` _rights) 10)
        (set `self.MilisecondsResults` (`self.PadSingleDigit` _rights))
        (else
          (set `self.MilisecondsResults` _rights))))
    (:`then_3`
      (return (`KismetStringLibrary.Concat_StrStr` (`self.MinutesResult`) " : " (`self.SecondsResults`) " : " (`self.MilisecondsResults`))))))

(fn `ConvertMilToResultsTime`
  (returns (Text :type String))
  (for _array_element (`self.LapTimes`)
    (set `self.ResultsMiliseconds` (+ (`self.ResultsMiliseconds`) _array_element))
    (bind _resulttext (`self.ConvertLapResults` _array_element))
    (`KismetArrayLibrary.Array_Add` (`self.LapResults`) _resulttext))
  (`|ExecutionSequence`
    (:`then_0`
      (bind _resulttext_2 (`self.ConvertLapResults` (`self.ResultsMiliseconds`)))
      (set `self.FinishResultsText` _resulttext_2))
    (:`then_1`
      (`KismetSystemLibrary.K2_ClearAndInvalidateTimerHandle` (`self.LapTimer`)))))

(fn `ConvertTimeToString`
  (returns (TimeText :type String))
  (return (`KismetStringLibrary.Concat_StrStr` (`KismetTextLibrary.Conv_TextToString` (`KismetTextLibrary.Conv_IntToText` (`self.Minutes`) false true 2)) " : " (`KismetTextLibrary.Conv_TextToString` (`KismetTextLibrary.Conv_IntToText` (`self.Seconds`) false true 2)) " : " (`KismetTextLibrary.Conv_TextToString` (`KismetTextLibrary.Conv_IntToText` (`self.Miliseconds`) false true 2)))))

(fn `DecreaseCountdown`
  (bind _countdownvalue (`self.CountdownValue`))
  (`Widget.SetVisibility` (`/Game/UI/WB_RaceHUD.TimerTxt` (`self.RacingHUD`)) "Visible")
  (if (< _countdownvalue 1)
    (`KismetSystemLibrary.K2_ClearAndInvalidateTimerHandle` (`self.CountdownTimer`))
    (`Widget.SetVisibility` (`/Game/UI/WB_RaceHUD.TimerTxt` (`self.RacingHUD`)) "Hidden")
    (`self.StartRace`)
    (else
      (`/Engine/EditorBlueprintResources/StandardMacros.DecrementInt` _countdownvalue))))

(fn `Get Highest Lap`
  (returns (HighestLap :type Integer))
  (`KismetArrayLibrary.Array_Clear` (`self.AllCurrentLaps`))
  (for _array_element (`self.AllRacers`)
    (`KismetArrayLibrary.Array_Add` (`self.AllCurrentLaps`) (`/Game/Vehicles/AI/BP_AIRacer.CurrentLap` _array_element)))
  (bind _output_get (set `self.HighestLap` (`.MaxValue` (`KismetMathLibrary.MaxOfIntArray` (`self.AllCurrentLaps`)))))
  (return _output_get))

(fn `Get Player Distance Index`
  (returns (Index :type Integer))
  (bind _aidistances (`self.AIDistances`))
  (for (_array_element _array_index) _aidistances
    (for _index (range _array_index (`KismetArrayLibrary.Array_Length` _aidistances))
      (if (> (`|GetArrayItem` (`self.AIDistances`) _index) _array_element)
        (`KismetArrayLibrary.Array_Swap` (`self.AIDistances`) _index _array_index))))
  (return (`KismetArrayLibrary.Array_Find` (`self.AIDistances`) (`/Game/Vehicles/Player/BP_Hoverbike.PlayerTotalDistance` (`self.Player`)))))

(fn `Get Racer Distance Along Spline`
  (params (Spline :type "SplineComponent Object Reference") (ActorLocation :type "Vector Structure"))
  (returns (Distance :type "Float (double-precision)"))
  (bind _returnvalue (`SplineComponent.FindInputKeyClosestToWorldLocation` Spline ActorLocation))
  (bind _returnvalue_2 (`KismetMathLibrary.FTrunc` _returnvalue))
  (bind _returnvalue_3 (`SplineComponent.GetDistanceAlongSplineAtSplinePoint` Spline _returnvalue_2))
  (`/Engine/EditorBlueprintResources/StandardMacros.IsValid` Spline
    (:`Is Valid`
      (return (+ _returnvalue_3 (* (- (`SplineComponent.GetDistanceAlongSplineAtSplinePoint` Spline (`KismetMathLibrary.FTrunc` (+ _returnvalue 1.0))) _returnvalue_3) (- _returnvalue (`KismetMathLibrary.Conv_IntToDouble` _returnvalue_2))))))))

(fn `GetLapResults`
  (bind _laptimes (`self.LapTimes`))
  (`KismetArrayLibrary.Array_Add` _laptimes (`self.LapTmeMiliseconds`))
  (if (> (`KismetArrayLibrary.Array_Length` _laptimes) 1)
    (if (< (`self.LapTmeMiliseconds`) (`self.BestTimeMiliseconds`))
      (set `self.BestTimeMiliseconds` (`self.LapTmeMiliseconds`) :!label _label)
      (set `self.BestTime` (`self.LapTime`)))
    (else
      (goto _label)))
  (set `self.PreviousTime` (`self.LapTime`))
  (`self.ResetLapTime`)
  (`/Engine/EditorBlueprintResources/StandardMacros.IncrementInt` (`self.PlayerCurrentLap`)))

(fn `GetPlayerPosition`
  (bind _player (`self.Player`))
  (bind _distance (`self.GetSplineTotalDistance`))
  (set `self.SplineDistance` _distance)
  (if (`/Game/Vehicles/Player/BP_Hoverbike.HasPlayerStarted` (`self.Player`))
    (`KismetArrayLibrary.Array_Clear` (`self.AIDistances`))
    (`KismetArrayLibrary.Array_Clear` (`self.AllRacerDistances`))
    (`self.Player`
      (:`then`
        (bind _highestlap (`self.Get Highest Lap`))
        (set `self.Highest Lap` _highestlap)
        (`|ExecutionSequence`
          (:`then_0`
            (bind _distance_2 (`self.Get Racer Distance Along Spline` (`self.TrackSpline`) (`self.K2_GetActorLocation` (`self.Player`))))
            (bind _output_get (set `self.PlayerDistance` _distance_2))
            (bind _output_get_2 (set `/Game/Vehicles/Player/BP_Hoverbike.PlayerTotalDistance` (+ _output_get (* (`self.PlayerCurrentLap`) (`self.SplineDistance`))) _player))
            (set `/Game/Vehicles/Player/BP_BasePawn.RacerDistance` _output_get_2 _player))
          (:`then_1`
            (for _array_element (`self.AllRacers`)
              (bind _distance_3 (`self.Get Racer Distance Along Spline` (`self.TrackSpline`) (`self.K2_GetActorLocation` _array_element)))
              (bind _returnvalue (+ _distance_3 (* (`/Game/Vehicles/AI/BP_AIRacer.CurrentLap` _array_element) (`self.SplineDistance`))))
              (`KismetArrayLibrary.Array_Add` (`self.AIDistances`) _returnvalue)
              (bind _output_get_3 (set `/Game/Vehicles/AI/BP_AIRacer.TotalTravelledDistance` _returnvalue _array_element))
              (set `/Game/Vehicles/Player/BP_BasePawn.RacerDistance` _output_get_3 _array_element))
            (`KismetArrayLibrary.Array_Add` (`self.AIDistances`) (`/Game/Vehicles/Player/BP_Hoverbike.PlayerTotalDistance` (`self.Player`)))
            (bind _index (`self.Get Player Distance Index`))
            (set `self.PlayerPosition` (+ _index 1)))))
      (:`else`
        (`KismetSystemLibrary.PrintString` "Player not valid")))
    (else
      (set `self.PlayerPosition` (+ (`KismetArrayLibrary.Array_Length` (`self.AllRacers`)) 1)))))

(fn `GetRacerPositions`
  (`self.SortDistances`))

(fn `GetSplineTotalDistance`
  (returns (Distance :type "Float (double-precision)"))
  (bind _output (`|GetArrayItem` (`self.AllRacers`)))
  (bind _spline (`/Game/Blueprints/BP_TrackSpline.Spline` (`/Game/Vehicles/AI/BP_AIRacer.CurrentTrackSpline` _output)))
  (`/Engine/EditorBlueprintResources/StandardMacros.IsValid` _output
    (:`Is Valid`
      (bind _output_get (set `self.TrackSpline` _spline))
      (return (`SplineComponent.GetDistanceAlongSplineAtSplinePoint` _output_get (- (`SplineComponent.GetNumberOfSplinePoints` _spline) 1))))))

(fn `ResetLapTime`
  (set `self.Miliseconds` 0)
  (set `self.Seconds` 0)
  (set `self.Minutes` 0)
  (set `self.LapTmeMiliseconds` 0))

(fn `SortDistances`
  (bind _distancesunsorted (`self.DistancesUnSorted`))
  (bind (_indexofmaxvalue _maxvalue) (`KismetMathLibrary.MaxOfFloatArray` _distancesunsorted))
  (`KismetArrayLibrary.Array_Clear` (`self.DistancesUnSorted`))
  (`KismetArrayLibrary.Array_Clear` (`self.DistancesSorted`))
  (`KismetArrayLibrary.Array_Clear` (`self.RacersSorted`))
  (`KismetArrayLibrary.Array_Clear` (`self.RacersUnsorted`))
  (set `self.RacersUnsorted` (`self.Racers`))
  (for _array_element (`self.Racers`)
    (`KismetArrayLibrary.Array_Add` (`self.DistancesUnSorted`) (`/Game/Vehicles/Player/BP_BasePawn.RacerDistance` _array_element)))
  (while (> (`KismetArrayLibrary.Array_Length` _distancesunsorted) 0)
    (`KismetArrayLibrary.Array_Add` (`self.DistancesSorted`) _maxvalue)
    (`KismetArrayLibrary.Array_AddUnique` (`self.RacersSorted`) (`|GetArrayItem` (`self.RacersUnsorted`) _indexofmaxvalue))
    (`KismetArrayLibrary.Array_Remove` (`self.RacersUnsorted`) _indexofmaxvalue)
    (`KismetArrayLibrary.Array_Remove` (`self.DistancesUnSorted`) _indexofmaxvalue))
  (for (_array_element_2 _array_index) (`self.RacersSorted`)
    (set `/Game/Vehicles/Player/BP_BasePawn.RacerPosition` (+ _array_index 1) _array_element_2)))

(fn `StartTimer`
  (bind _miliseconds (`self.Miliseconds`))
  (if (not (`self.IsRaceFinished`))
    (`|ExecutionSequence`
      (:`then_0`
        (`/Engine/EditorBlueprintResources/StandardMacros.IncrementInt` _miliseconds
          (:`  `
            (`/Engine/EditorBlueprintResources/StandardMacros.IncrementInt` (`self.LapTmeMiliseconds`)
              (:`  `
                (if (> _miliseconds 99)
                  (`/Engine/EditorBlueprintResources/StandardMacros.IncrementInt` (`self.Seconds`)
                    (:`  `
                      (set `self.Miliseconds` 0)
                      (if (> (`self.Seconds`) 59)
                        (`/Engine/EditorBlueprintResources/StandardMacros.IncrementInt` (`self.Minutes`)
                          (:`  `
                            (set `self.Seconds` 0))))))))))))
      (:`then_1`
        (bind _timetext (`self.ConvertTimeToString`))
        (set `self.LapTime` _timetext)))))

(fn `UserConstructionScript`)