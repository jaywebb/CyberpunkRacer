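; BP_FinishMarker is the finish line trigger that counts laps and ends the race.
; AI racers overlapping its box gain a lap only after reaching a checkpoint.
; Player crossings record lap results through the game mode's TimeKeeper, gated by an enabled flag and DoOnce that EnableLapCollision re-arms; otherwise they mark the player as started.
; On the final lap it stops position timers, halts all racers and converts the results time.
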(event `self.ReceiveBeginPlay`)

(event `EnableLapCollision`
  (set `self.IsEnabled` true)
  (goto _label :!via `Reset`))

(event `self.Box.OnComponentBeginOverlap`
  (params (OverlappedComponent :type "PrimitiveComponent Object Reference") (OtherActor :type "Actor Object Reference") (OtherComp :type "PrimitiveComponent Object Reference") (OtherBodyIndex :type Integer) (bFromSweep :type Boolean) (SweepResult :type "HitResult Structure (by ref)"))
  (bind _asbp_airacer (cast `/Game/Vehicles/AI/BP_AIRacer` OtherActor)
    (:`then`
      (if (`/Game/Vehicles/AI/BP_AIRacer.HasReachedCheckpoint` _asbp_airacer)
        (`/Game/Vehicles/AI/BP_AIRacer.AddToLapCount` _asbp_airacer)
        (set `/Game/Vehicles/AI/BP_AIRacer.HasReachedCheckpoint` false _asbp_airacer)))
    (:`CastFailed`
      (bind _asbp_hoverbike (cast `/Game/Vehicles/Player/BP_PlayerRacer` OtherActor))
      (if (`self.IsEnabled`)
        (bind _timekeeper (`/Game/Blueprints/RacingGameMode.TimeKeeper` (`/Game/Vehicles/Player/BP_PlayerRacer.As Racing Game Mode` _asbp_hoverbike)))
        (set `self.Time Keeper` _timekeeper)
        (`/Engine/EditorBlueprintResources/StandardMacros.DoOnce` false :!label _label
          (:`Completed`
            (`/Game/Blueprints/BP_TimeKeeper.GetLapResults` _timekeeper)
            (set `self.IsEnabled` false)
            (if (== (`/Game/Blueprints/BP_TimeKeeper.PlayerCurrentLap` _timekeeper) (`self.LapCountToFinish`))
              (`KismetSystemLibrary.K2_ClearAndInvalidateTimerHandle` (`/Game/Blueprints/BP_TimeKeeper.PositionTimer` _timekeeper))
              (`KismetSystemLibrary.K2_ClearAndInvalidateTimerHandle` (`/Game/Blueprints/BP_TimeKeeper.AIPositionTimer` _timekeeper))
              (set `/Game/Blueprints/BP_TimeKeeper.IsRaceFinished` true _timekeeper)
              (set `/Game/Vehicles/Player/BP_PlayerRacer.Current speed` 0.0 _asbp_hoverbike)
              (set `/Game/Vehicles/Player/BP_PlayerRacer.IsMovementEnabled?` false _asbp_hoverbike)
              (`/Game/Blueprints/BP_TimeKeeper.ConvertMilToResultsTime` _timekeeper)
              (bind _outactors (`GameplayStatics.GetAllActorsOfClass` "/Game/Vehicles/AI/BP_AIRacer.BP_AIRacer_C"))
              (for _array_element _outactors
                (set `/Game/Vehicles/AI/BP_AIRacer.MaxSpeed` 0.0 _array_element)
                (set `/Game/Vehicles/AI/BP_AIRacer.IsEnabled` false _array_element)))))
        (else
          (set `/Game/Vehicles/Player/BP_PlayerRacer.HasPlayerStarted` true _asbp_hoverbike))))))

(fn `UserConstructionScript`)