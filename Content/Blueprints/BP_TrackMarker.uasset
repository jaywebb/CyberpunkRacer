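; BP_TrackMarker is a placeable track marker holding track data, apparently intended for BP_AIRacer actors.
; Its construction script snaps it to the closest point on the referenced track's spline, when valid, and places two cubes at plus and minus OffsetMax on local X.
; The sphere overlap events are empty.
; The nodes that would reset a racer's marker or pass it the track data are disconnected and never run.
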(event `self.Sphere.OnComponentBeginOverlap`
  (params (OverlappedComponent :type "PrimitiveComponent Object Reference") (OtherActor :type "Actor Object Reference") (OtherComp :type "PrimitiveComponent Object Reference") (OtherBodyIndex :type Integer) (bFromSweep :type Boolean) (SweepResult :type "HitResult Structure (by ref)")))

(event `self.Sphere.OnComponentEndOverlap`
  (params (OverlappedComponent :type "PrimitiveComponent Object Reference") (OtherActor :type "Actor Object Reference") (OtherComp :type "PrimitiveComponent Object Reference") (OtherBodyIndex :type Integer)))

(fn `UserConstructionScript`
  (bind (_newtrackdata_maxspeed _newtrackdata_speedchangerate _newtrackdata_offsetmax) (break `/Game/Blueprints/TrackMarkerData` (`self.NewTrackData`)))
  (bind _trackref (`self.TrackRef`)
    (:`then`
      (bind _returnvalue_location (`KismetMathLibrary.BreakTransform` (`SplineComponent.FindTransformClosestToWorldLocation` (`/Game/Blueprints/BP_TrackSpline.Spline` _trackref) (`self.K2_GetActorLocation`) "World" false)))
      (`self.K2_SetActorLocation` _returnvalue_location)
      (`SceneComponent.K2_SetRelativeLocation` (`self.Cube`) (`KismetMathLibrary.MakeVector` _newtrackdata_offsetmax) false false)
      (`SceneComponent.K2_SetRelativeLocation` (`self.Cube1`) (`KismetMathLibrary.MakeVector` (* _newtrackdata_offsetmax -1.0)) false false))
    (:`else`)))