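; AI racer bike that follows the track spline and registers itself with the game's TimeKeeper and racing HUD.
; Tick sweeps it forward, eases speed toward MaxSpeed, interpolates onto the spline at a lateral offset, and pitches it from a ground trace.
; Track markers set speed and lane limits, while a timer re-rolls MaxSpeed scaled by race position.
; Obstacle dodging, hit response and random lane changes exist but are disconnected.
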(event `DodgeCollision`
  (params (Direction :type "Float (double-precision)"))
  (bind _returnvalue (+ (`self.ActorRightOffset`) 250.0))
  (bind _returnvalue_2 (- (`self.ActorRightOffset`) 249.0))
  ;[1 0.7407 0.3582] Dodge Collisions
  (set `self.SideDirection` Direction)
  (set `self.IsMovingSideways` true)
  (`/Engine/EditorBlueprintResources/StandardMacros.DoOnce` false :!label _label
    (:`Completed`
      (`|ExecutionSequence`
        (:`then_0`
          (`/Engine/EditorBlueprintResources/StandardMacros.CompareFloat` (`self.SideDirection`) 1.0
            (:`>`
              (if (> _returnvalue (`self.OffsetMax`))
                (set `self.ActorRightOffset` 1.0 :!label _label_2)
                (else
                  (set `self.ActorRightOffset` _returnvalue))))
            (:`<`
              (if (< _returnvalue_2 (`self.OffsetMin`))
                (goto _label_2)
                (else
                  (set `self.ActorRightOffset` _returnvalue_2))))))
        (:`then_1`
          (if (> (`self.CurrentSpeed`) 1000.0)
            (`KismetSystemLibrary.Delay` 0.2)
            (else
              (`KismetSystemLibrary.Delay` 1.0)))
          (set `self.IsMovingSideways` false)
          (`self.ResetDodge`))))))

(event `ResetDodge`
  ;[1 0.7407 0.3582] Dodge Collisions
  (goto _label :!via `Reset`))

(event `self.ReceiveBeginPlay`
  (bind (_returnvalue_roll _returnvalue_pitch) (`KismetMathLibrary.BreakRotator` (`SceneComponent.K2_GetComponentRotation` (`self.ForwardDirection`))))
  (`|ExecutionSequence`
    (:`then_0`
      (`self.SetRacerIDs`))
    (:`then_1`
      (set `self.Return Value Y (Pitch)` _returnvalue_pitch)
      (`KismetSystemLibrary.K2_SetTimer` null "AdjustSpeed" 6.0 true)
      (`KismetSystemLibrary.K2_SetTimer` null "Set Bike Lane" 2.0 true)
      (`SceneComponent.SetVisibility` (`self.TextRender`) true false)
      (set `self.MaxSpeed` 3000.0))))

(event `ProcessTrackMarker`
  (params (NewTrackData :type "/Game/Blueprints/TrackMarkerData Structure"))
  (bind (_maxspeed _speedchangerate _offsetmax) (break `/Game/Blueprints/TrackMarkerData` NewTrackData))
  (`/Engine/EditorBlueprintResources/StandardMacros.DoOnce` false :!label _label_3
    (:`Completed`
      (set `self.MaxSpeed` _maxspeed)
      (set `self.SpeedChangeRate` _speedchangerate)
      (set `self.OffsetMax` _offsetmax)
      (set `self.OffsetMin` (* _offsetmax -1.0)))))

(event `ResetMarker`
  (goto _label_3 :!via `Reset`))

(event `HitObjectCooldown`
  (`/Engine/EditorBlueprintResources/StandardMacros.DoOnce` false :!label _label_4
    (:`Completed`
      (`KismetSystemLibrary.K2_SetTimer` null "ResetHitObject" 3.0))))

(event `ResetCooldown`
  (goto _label_4 :!via `Reset`))

(event `self.ReceiveTick`
  (params (DeltaSeconds :type "Float (single-precision)"))
  (bind _forwarddirection (`self.ForwardDirection`))
  (bind (_returnvalue_roll _returnvalue_pitch _returnvalue_yaw) (`KismetMathLibrary.BreakRotator` (`SceneComponent.K2_GetComponentRotation` _forwarddirection)))
  (if (`self.HoldInPlace`)
    (set `self.CurrentSpeed` 0.0)
    (else
      (`self.K2_AddActorLocalOffset` (+ (`KismetMathLibrary.MakeVector` (* DeltaSeconds (`self.CurrentSpeed`))) (`SceneComponent.GetForwardVector` (`self.ForwardDirection`))) true true) ; Sweep plane forwards
      (`self.MaintainSpeed`)
      (`self.FollowSpline`)
      (`self.AdjustBikeRotation`)
      (`SceneComponent.K2_SetWorldRotation` _forwarddirection (`KismetMathLibrary.MakeRotator` _returnvalue_roll (`self.Return Value Y (Pitch)`) _returnvalue_yaw) false false))))

(event `self.ReceiveHit`
  (params (MyComp :type "PrimitiveComponent Object Reference") (Other :type "Actor Object Reference") (OtherComp :type "PrimitiveComponent Object Reference") (bSelfMoved :type Boolean) (HitLocation :type "Vector Structure") (HitNormal :type "Vector Structure") (NormalImpulse :type "Vector Structure") (Hit :type "HitResult Structure (by ref)")))

(event `AddToLapCount`
  (`/Engine/EditorBlueprintResources/StandardMacros.DoOnce` false :!label _label_5
    (:`Completed`
      (`/Engine/EditorBlueprintResources/StandardMacros.IncrementInt` (`self.CurrentLap`)))))

(event `ResetLapFinishOverlap`
  (goto _label_5 :!via `Reset`))

(fn `AdjustBikeRotation`
  (bind (_returnvalue_roll _returnvalue_pitch _returnvalue_yaw) (`KismetMathLibrary.BreakRotator` (`self.K2_GetActorRotation`)))
  (bind (_returnvalue_roll_2 _returnvalue_pitch_2) (`KismetMathLibrary.BreakRotator` (`self.K2_GetActorRotation`)))
  (bind _hoverpoint (`self.HoverPoint`))
  (bind (_returnvalue_x _returnvalue_y _returnvalue_z) (`KismetMathLibrary.BreakVector` (`SceneComponent.K2_GetComponentLocation` _hoverpoint)))
  (bind _outhit (`KismetSystemLibrary.LineTraceSingle` (`SceneComponent.K2_GetComponentLocation` _hoverpoint) (`KismetMathLibrary.MakeVector` _returnvalue_x _returnvalue_y (- _returnvalue_z 10000.0)) "TraceTypeQuery1"))
  (bind (_returnvalue_roll_3 _returnvalue_pitch_3) (`KismetMathLibrary.BreakRotator` (`KismetMathLibrary.Conv_VectorToRotator` (`.Normal` (`GameplayStatics.BreakHitResult` _outhit)))))
  (bind (_returnvalue_roll_4 _returnvalue_pitch_4) (`KismetMathLibrary.BreakRotator` (`KismetMathLibrary.MakeRotator` 0.0 (* (- _returnvalue_pitch_3 90.0) -1.0))))
  (set `self.SurfaceRotation` (`KismetMathLibrary.FInterpTo` (`self.SurfaceRotation`) (`KismetMathLibrary.FClamp` _returnvalue_pitch_4 0.0 25.0) (`GameplayStatics.GetWorldDeltaSeconds`) 2.0))
  (`self.K2_SetActorRotation` (`KismetMathLibrary.MakeRotator` _returnvalue_roll (+ (* _returnvalue_pitch_2 -0.025) (`self.SurfaceRotation`)) _returnvalue_yaw)))

(fn `AdjustSpeed`
  (if (`self.IsEnabled`)
    (set `self.MaxSpeed` (`KismetMathLibrary.FClamp` (* (`KismetMathLibrary.RandomIntegerInRange` 4 10) (* (`self.RacerPosition`) 200)) 2000.0 5000.0))))

(fn `CheckCollisions`
  (bind _forwardpoint (`self.ForwardPoint`))
  (bind _returnvalue (+ (* (`SceneComponent.GetForwardVector` _forwardpoint) (`self.ForwardCollisionDistance`)) (`SceneComponent.K2_GetComponentLocation` _forwardpoint)))
  (bind _outhit (`KismetSystemLibrary.BoxTraceSingle` _returnvalue _returnvalue (500.0 50.0 50.0) (`SceneComponent.K2_GetComponentRotation` _forwardpoint) "TraceTypeQuery1"))
  (bind (_bblockinghit _binitialoverlap _time _distance _location _impactpoint _normal _impactnormal _physmat _hitactor) (`GameplayStatics.BreakHitResult` _outhit))
  (bind _asbp_base_pawn (cast `/Game/Vehicles/Player/BP_BasePawn` _hitactor)
    (:`then`
      (set `self.HitLocation` (`SceneComponent.K2_GetComponentLocation` (`/Game/Vehicles/Player/BP_BasePawn.Box` _asbp_base_pawn)))
      (set `self.IsForwardBlocked` true :!label _label)
      (set `self.DistanceToForwardCollision` (`KismetMathLibrary.VSize` (- (`SceneComponent.K2_GetComponentLocation` (`self.Biker`)) (`self.HitLocation`))))
      (`self.CheckSideCollisions`))
    (:`CastFailed`
      (cast `/Game/Blueprints/BP_Obstacle` _hitactor
        (:`then`
          (set `self.HitLocation` _location)
          (goto _label))
        (:`CastFailed`
          (set `self.IsForwardBlocked` false)
          (set `self.DistanceToForwardCollision` 3000.0))))))

(fn `CheckSideCollisions`
  (bind _sidecollisionpt (`self.SideCollisionPt`))
  (bind _returnvalue (+ (* (`SceneComponent.GetRightVector` _sidecollisionpt) (* (`self.LeftCollisionDistance`) (`self.SideCollisionModifier`))) (`SceneComponent.K2_GetComponentLocation` _sidecollisionpt)))
  (if (not (`self.IsMovingSideways`))
    (`|ExecutionSequence`
      (:`then_0`
        (set `self.SideCollisionPt` (`self.LeftOffsetPosition`))
        (set `self.SideCollisionModifier` -1.0))
      (:`then_1`
        (set `self.SideCollisionPt` (`self.RightOffsetPosition`))
        (set `self.SideCollisionModifier` 1.0)))
    (bind _outhit (`KismetSystemLibrary.BoxTraceSingle` _returnvalue _returnvalue (200.0 50.0 50.0) (`SceneComponent.K2_GetComponentRotation` _sidecollisionpt) "TraceTypeQuery1"))
    (cast `/Game/Vehicles/Player/BP_BasePawn` (`.HitActor` (`GameplayStatics.BreakHitResult` _outhit))
      (:`then`
        (set `self.IsSideMovementBlocked` true))
      (:`CastFailed`
        (set `self.IsSideMovementBlocked` false)
        (`self.DodgeCollision` (`self.SideCollisionModifier`))))))

(fn `FollowSpline`
  (bind _returnvalue_location (`KismetMathLibrary.BreakTransform` (`self.GetTransform`)))
  (bind _currenttrackspline (`self.CurrentTrackSpline`)
    (:`then`
      (bind (_returnvalue_location_2 _returnvalue_rotation) (`KismetMathLibrary.BreakTransform` (`SplineComponent.FindTransformClosestToWorldLocation` (`/Game/Blueprints/BP_TrackSpline.Spline` _currenttrackspline) (`self.K2_GetActorLocation`) "World" false)))
      (set `self.Direction` (`KismetMathLibrary.GetForwardVector` _returnvalue_rotation))
      (`self.K2_SetActorLocation` (`KismetMathLibrary.VInterpTo` _returnvalue_location (+ _returnvalue_location_2 (* (`KismetMathLibrary.GetRightVector` _returnvalue_rotation) (`self.ActorRightOffset`))) (`GameplayStatics.GetWorldDeltaSeconds`) 6.0) true true)
      (if (`self.HitObject`)
        (`self.HitObjectCooldown`)
        (else
          (`self.K2_SetActorRotation` (`KismetMathLibrary.RInterpTo` (`self.K2_GetActorRotation`) _returnvalue_rotation (`GameplayStatics.GetWorldDeltaSeconds`) 6.0) true))))
    (:`else`)))

(fn `GetBikeOffset`
  (switch `/Game/Blueprints/OffsetPositions` (`self.CurrentOffsetPosition`)
    (:`NewEnumerator0`
      (set `self.RelativeOffsetLocation` 0.0))
    (:`NewEnumerator1`
      (set `self.OffsetModifer` 1.0)
      (set `self.RelativeOffsetLocation` (`KismetMathLibrary.FClamp` (* 0.0 (`self.OffsetModifer`)) -1000.0 1000.0) :!label _label))
    (:`NewEnumerator2`
      (set `self.OffsetModifer` -1.0)
      (goto _label))))

(fn `MaintainSpeed`
  (set `self.MaxSpeedModifier` 1.0)
  (set `self.CurrentSpeed` (`KismetMathLibrary.FInterpTo` (`self.CurrentSpeed`) (`self.MaxSpeed`) (`GameplayStatics.GetWorldDeltaSeconds`) (`self.SpeedChangeRate`))))

(fn `OffsetLocation`
  (bind _sphere1 (`self.Sphere1`))
  (bind (_relativelocation_x _relativelocation_y) (`KismetMathLibrary.BreakVector` (`SceneComponent.RelativeLocation` _sphere1)))
  (if (> (`self.CurrentSpeed`) 0.0)
    (`SceneComponent.K2_SetRelativeLocation` _sphere1 (`KismetMathLibrary.MakeVector` 0.0 (`KismetMathLibrary.FClamp` (`KismetMathLibrary.FInterpTo` _relativelocation_y (`self.RelativeOffsetLocation`) (`GameplayStatics.GetWorldDeltaSeconds`) 6.0) (`self.OffsetMin`) (`self.OffsetMax`))) true true)))

(fn `ResetHitObject`
  (set `self.HitObject` false)
  (`self.ResetCooldown`))

(fn `ReturnFromHitRotation`
  (if (== (`self.HitRacerRef`) null)
    (`SceneComponent.K2_SetRelativeRotation` (`self.Sphere1`) (`KismetMathLibrary.RInterpTo` (`SceneComponent.RelativeRotation` (`self.Sphere1`)) (struct) (`GameplayStatics.GetWorldDeltaSeconds`) 1.0) false false)))

(fn `ReturnToCenter`)

(fn `Set Bike Lane`)

(fn `SetRacerIDs`
  (bind _returnvalue (- (`self.RacerID`) 1))
  (bind _racinghud (`/Game/Blueprints/BP_TimeKeeper.RacingHUD` (`self.TimeKeeper`)))
  (bind _asracing_game_mode (cast `/Game/Blueprints/RacingGameMode` (`GameplayStatics.GetGameMode`)))
  (set `self.TimeKeeper` (`/Game/Blueprints/RacingGameMode.TimeKeeper` _asracing_game_mode))
  (switch `int` _returnvalue
    (:`0`
      (set `/Game/UI/WB_RaceHUD.RacerRef1` self _racinghud))
    (:`1`
      (set `/Game/UI/WB_RaceHUD.RacerRef2` self _racinghud))
    (:`2`
      (set `/Game/UI/WB_RaceHUD.RacerRef3` self _racinghud))
    (:`3`
      (set `/Game/UI/WB_RaceHUD.RacerRef4` self _racinghud)))
  (`KismetArrayLibrary.Array_Set` (`/Game/Blueprints/BP_TimeKeeper.AllRacers` (`self.TimeKeeper`)) _returnvalue self true))

(fn `UserConstructionScript`
  (bind _biker (`self.Biker`))
  (set `SceneComponent.bAbsoluteScale` true _biker)
  (set `SceneComponent.bAbsoluteScale` true _biker)
  (`TextRenderComponent.K2_SetText` (`self.TextRender`) (`KismetTextLibrary.Conv_IntToText` (`self.RacerID`)))
  (bind _asbp_biker (cast `/Game/Vehicles/Player/BP_Biker` (`ChildActorComponent.ChildActor` (`self.Biker`))))
  (`/Game/Vehicles/Player/BP_Biker.SetBikerColor` _asbp_biker (`self.BikerColor`))
  (if (`self.Refresh?`)
    (`self.K2_SetActorLocation` (`SplineComponent.GetLocationAtSplinePoint` (`/Game/Blueprints/BP_TrackSpline.Spline` (`self.CurrentTrackSpline`)) (`self.Point Index`) "World"))))