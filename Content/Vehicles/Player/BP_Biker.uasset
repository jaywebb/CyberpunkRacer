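; BP_Biker is a player vehicle Blueprint for a rider and hoverbike that can be recolored.
; SetBikerColor stores the given color, then creates dynamic material instances for two SkeletalMesh slots and one Hoverbike2 slot.
; It applies that color as Tint on the Quinn material and as Color on both bike-material instances.
; The event graph and construction script are empty, so the function is not called within this file.
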(fn `SetBikerColor`
  (params (BikerColor :type "LinearColor Structure"))
  (bind _skeletalmesh (`self.SkeletalMesh`))
  (set `self.BikerColor` BikerColor)
  (bind _returnvalue (`PrimitiveComponent.CreateDynamicMaterialInstance` _skeletalmesh 1 "/Game/Characters/Mannequins/Materials/Instances/Quinn/MI_Quinn_03.MI_Quinn_03" "None"))
  (`MaterialInstanceDynamic.SetVectorParameterValue` _returnvalue "Tint" (`self.BikerColor`))
  (bind _returnvalue_2 (`PrimitiveComponent.CreateDynamicMaterialInstance` _skeletalmesh 0 "/Game/Vehicles/AI/BikeMat1_Inst.BikeMat1_Inst" "None"))
  (`MaterialInstanceDynamic.SetVectorParameterValue` _returnvalue_2 "Color" (`self.BikerColor`))
  (bind _returnvalue_3 (`PrimitiveComponent.CreateDynamicMaterialInstance` (`self.Hoverbike2`) 0 "/Game/Vehicles/AI/BikeMat1_Inst.BikeMat1_Inst" "None"))
  (`MaterialInstanceDynamic.SetVectorParameterValue` _returnvalue_3 "Color" (`self.BikerColor`)))

(fn `UserConstructionScript`)